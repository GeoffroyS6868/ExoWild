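; Game instance for Exowild that holds player stats, skills and session flags, and persists player data to a save slot.
; On Init it creates the save if none exists, then loads it and caches stats and skills.
; SavePlayerData updates the cache and writes a fresh BP_Save object to the slot.
; Gamepad-use and intro-seen flags have getters and setters but are not saved.
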(event Custom|Save
  (bind _returnvalue (SaveGame|CreateSaveGameObject "/Game/Blueprint/Core/Save/BP_Save.BP_Save_C"))
  (Default|SaveData _returnvalue (Variables|Default|GetSkills) (Variables|Default|GetPlayerStats))
  (SaveGame|SaveGametoSlot _returnvalue "Exowild"))

(event EventInit
  (bind _returnvalue (SaveGame|DoesSaveGameExist "Exowild"))
  (if _returnvalue
    _
    (else
      (bind _returnvalue_2 (SaveGame|CreateSaveGameObject "/Game/Blueprint/Core/Save/BP_Save.BP_Save_C"))
      (SaveGame|SaveGametoSlot _returnvalue_2 "Exowild")))
  (bind _returnvalue_3 (SaveGame|LoadGamefromSlot "Exowild"))
  (bind _asbp_save (Utilities|Casting|CastToBP_Save _returnvalue_3))
  (Variables|Default|SetPlayerStats (Variables|/Game/Blueprint/Core/Save/BP_Save.BP_Save_C|GetPlayerStats _asbp_save))
  (Variables|Default|SetSkills (Variables|/Game/Blueprint/Core/Save/BP_Save.BP_Save_C|GetSkills _asbp_save)))

(fn SetIsUsingGamepad
  (params (IsUsingGamepad :type Boolean))
  (Variables|Default|SetIsUsingGamepad IsUsingGamepad))

(fn GetIsUsingGamepad
  (return (Variables|Default|GetIsUsingGamepad)))

(fn SetHasSeentheIntro
  (params (HasSeenTheIntro :type Boolean))
  (Variables|Default|SetHasSeenTheIntro HasSeenTheIntro))

(fn GetHasSeentheIntro
  (return (Variables|Default|GetHasSeenTheIntro)))

(fn SavePlayerData
  (params (PlayerStats :type BPS%20Player%20Stats%20Structure) (Skills :type Array%20of%20Names))
  (Variables|Default|SetPlayerStats PlayerStats)
  (Variables|Default|SetSkills Skills)
  (CallFunction|Save))

(fn GetPlayerData
  (return (Variables|Default|GetPlayerStats) (Variables|Default|GetSkills)))