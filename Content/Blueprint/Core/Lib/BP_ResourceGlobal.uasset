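; BP_ResourceGlobal is a set of lookup helpers that map a resource enum value to its drop actor and its icon.
; Both functions convert the enum to a row name and read that row from the DT_Resources data table, returning its Drop or Icon field.
; A missing row falls back to the rock defaults, BP_Rock for the actor and ICON_Rock for the icon.
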(fn GetActorfromResource
  (params (Resource :type E_Resources%20Enum :default "NewEnumerator0"))
  (bind _returnvalue (Utilities|GetDataTableRow "/Game/Blueprint/Core/DataTables/DT_Resources.DT_Resources" (Utilities|String|StringToName (Utilities|String|EnumtoString Resource)))
    (:then
      (return (.drop _returnvalue)))
    (:RowNotFound
      (return "/Game/Blueprint/Actor/Resources/BP_Rock.BP_Rock_C"))))

(fn GetIconfromResource
  (params (Resource :type E_Resources%20Enum :default "NewEnumerator0"))
  (bind _returnvalue (Utilities|GetDataTableRow "/Game/Blueprint/Core/DataTables/DT_Resources.DT_Resources" (Utilities|String|StringToName (Utilities|String|EnumtoString Resource)))
    (:then
      (return (.icon _returnvalue)))
    (:RowNotFound
      (return "/Game/Assets/UI/ResourcesIcon/ICON_Rock.ICON_Rock"))))