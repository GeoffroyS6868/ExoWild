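; Global skill helper library for looking up skills, describing their stat bonuses and tracking which ones the player has unlocked.
; Skill rows come from DT_Skills by name, and bonus text joins each stat's name, value and optional percent symbol from parallel arrays.
; Unlock state lives in the Skills array on player 0's BP_MainCharacter, and a skill named "None" always counts as unlocked.
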(fn GetSkillfromName
  (params (Name :type Name))
  (bind _returnvalue (Utilities|GetDataTableRow "/Game/Blueprint/Core/DataTables/DT_Skills.DT_Skills" Name)
    (:then
      (return _returnvalue))
    (:RowNotFound
      (return ""))))

(fn CreateBonusText
  (params (Stats :type Array%20of%20E_Stats%20Enums :default "NewEnumerator0") (Bonus :type Array%20of%20Integers))
  (for (_array_element _array_index) Stats
    (bind _name (CallFunction|GetStatsName _array_element))
    (LocalVariables|SetTest (Utilities|String|Append (LocalVariables|GetTest) _name " +" (Utilities|String|ToString(Integer) (Utilities|Array|Get(acopy) Bonus _array_index))))
    (bind _symbol (CallFunction|GetStatsSymbol _array_element))
    (LocalVariables|SetTest (Utilities|String|Append (LocalVariables|GetTest) _symbol " ")))
  (return (Utilities|Text|ToText(String) (LocalVariables|GetTest))))

(fn GetStatsSymbol
  (params (Stat :type E_Stats%20Enum :default "NewEnumerator0"))
  (switch Utilities|FlowControl|Switch|SwitchonE_Stats Stat
    (:NewEnumerator0
      _)
    (:NewEnumerator1
      (return "%"))
    (:NewEnumerator2
      _)
    (:NewEnumerator3
      _)
    (:NewEnumerator4
      _)
    (:NewEnumerator5
      (return "%"))
    (:NewEnumerator6
      (return "%")))
  (return ""))

(fn GetStatsName
  (params (Stat :type E_Stats%20Enum :default "NewEnumerator0"))
  (switch Utilities|FlowControl|Switch|SwitchonE_Stats Stat
    (:NewEnumerator0
      (return "Life"))
    (:NewEnumerator1
      (return "Regeneration"))
    (:NewEnumerator2
      (return "Defense"))
    (:NewEnumerator3
      (return "Gun Damage"))
    (:NewEnumerator4
      (return "Kick Damage"))
    (:NewEnumerator5
      (return "Speed"))
    (:NewEnumerator6
      (return "Resource Bonus"))))

(fn HasUnlocked
  (params (SkillName :type Name))
  (if (== SkillName "")
    (return true)
    (else
      (bind _asbp_main_character (Utilities|Casting|CastToBP_MainCharacter (Game|Player|GetPlayerPawn 0))
        (:then
          (bind _array_element (Utilities|Array|ForEachLoopwithBreak (Variables|/Game/Blueprint/Character/BP_MainCharacter.BP_MainCharacter_C|GetSkills _asbp_main_character))
            (:LoopBody
              (if (== _array_element SkillName)
                (return true)))
            (:Completed
              (return false))))
        (:CastFailed
          (return false))))))

(fn AddSkilltoUnlocked
  (params (SkillName :type Name))
  (bind _asbp_main_character (Utilities|Casting|CastToBP_MainCharacter (Game|Player|GetPlayerPawn 0)))
  (Utilities|Array|Add (Variables|/Game/Blueprint/Character/BP_MainCharacter.BP_MainCharacter_C|GetSkills _asbp_main_character) SkillName))