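; BP_Settings is a Blueprint that exposes Exowild player state flags for gamepad use and whether the intro has been seen.
; It provides getter and setter pairs for each flag.
; Each function casts the game instance to BP_ExowildGameInstance and forwards the call, so the values live on the game instance rather than in this asset.
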(fn SetIsUsingGamepad
  (params (IsUsingGamepad :type Boolean))
  (bind _asbp_exowild_game_instance (Utilities|Casting|CastToBP_ExowildGameInstance (Game|GetGameInstance)))
  (Default|SetIsUsingGamepad _asbp_exowild_game_instance IsUsingGamepad))

(fn GetIsUsingGamepad
  (bind _asbp_exowild_game_instance (Utilities|Casting|CastToBP_ExowildGameInstance (Game|GetGameInstance)))
  (bind _isusinggamepad (Default|GetIsUsingGamepad _asbp_exowild_game_instance))
  (return _isusinggamepad))

(fn SetHasSeentheIntro
  (params (HasSeenTheIntro :type Boolean))
  (bind _asbp_exowild_game_instance (Utilities|Casting|CastToBP_ExowildGameInstance (Game|GetGameInstance)))
  (Default|SetHasSeentheIntro _asbp_exowild_game_instance HasSeenTheIntro))

(fn GetHasSeentheIntro
  (bind _asbp_exowild_game_instance (Utilities|Casting|CastToBP_ExowildGameInstance (Game|GetGameInstance)))
  (bind _hasseen (Default|GetHasSeentheIntro _asbp_exowild_game_instance))
  (return _hasseen))