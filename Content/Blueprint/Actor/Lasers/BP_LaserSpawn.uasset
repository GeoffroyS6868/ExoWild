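; BP_LaserSpawn is a laser emitter actor that fires a short-lived BP_Laser from its Arrow component.
; On BeginPlay it picks Laser_Push audio for non-red colors, spawns the laser with its color and a self-reference, then destroys its lasers and itself after a brief delay.
; An Update event clears the tracked ChildLasers and respawns the beam from the emitter's current transform.
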(event Custom|Update
  (CallFunction|DestroyChilds)
  (bind _returnvalue (Game|SpawnActorfromClass "/Game/Blueprint/Actor/Lasers/BP_Laser.BP_Laser_C" (Math|Transform|MakeTransform (Transformation|GetWorldLocation (Variables|Default|GetArrow)) (Transformation|GetActorRotation) "1.000000,1.000000,1.000000") "Undefined" "MultiplyWithRoot" 0 (Variables|Default|GetLaserColor) (Variables|Default|GetSpawnReference) 0))
  (Utilities|Array|Add (Variables|Default|GetChildLasers) _returnvalue))

(event EventBeginPlay
  (bind _self self)
  (if (== (Variables|Default|GetLaserColor) "(R=1.000000,G=0.000000,B=0.000000,A=1.000000)")
    _
    (else
      (Audio|Components|Audio|SetSound (Variables|Default|GetAudio) "/Game/Assets/Sounds/Effects/Laser_Push.Laser_Push")))
  (Variables|Default|SetSpawnReference _self)
  (Variables|Default|SetID (Utilities|GetDisplayName _self))
  (bind _returnvalue (Game|SpawnActorfromClass "/Game/Blueprint/Actor/Lasers/BP_Laser.BP_Laser_C" (Math|Transform|MakeTransform (Transformation|GetWorldLocation (Variables|Default|GetArrow)) (Transformation|GetActorRotation) "1.000000,1.000000,1.000000") "Undefined" "MultiplyWithRoot" 0 (Variables|Default|GetLaserColor) (Variables|Default|GetSpawnReference) 0))
  (Utilities|Array|Add (Variables|Default|GetChildLasers) _returnvalue)
  (Components|Activation|Activate (Variables|Default|GetAudio) false)
  (Utilities|FlowControl|Delay 0.1)
  (CallFunction|DestroyChilds)
  (Actor|DestroyActor))

(fn ConstructionScript
  (|CallParentFunction))

(fn DestroyChilds
  (for _array_element (Variables|Default|GetChildLasers)
    (Actor|DestroyActor _array_element))
  (Utilities|Array|Clear (Variables|Default|GetChildLasers)))