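; BP_Ore is a damageable ore actor that drops a resource when destroyed.
; Its Damage event subtracts from Life and calls DropResources once Life reaches zero or below.
; DropResources looks up the actor class for the ore's Type, spawns it at an offset along the ore's local up axis regardless of collision, then destroys the ore.
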(event Custom|DropResources
  ;[0.1 0.1 0.1] Drop Rersources
  (bind _newparam (CallFunction|GetActorfromResource (Variables|Default|GetType)))
  (Game|SpawnActorfromClass _newparam (Math|Transform|MakeTransform (+ (Transformation|GetActorLocation) (Math|Vector|RotateVector (Math|Vector|MakeVector 0.0 0.0 2e+02) (Transformation|GetActorRotation))) "0, 0, 0" "1.000000,1.000000,1.000000") "AlwaysSpawn" "MultiplyWithRoot" 0 0)
  (Actor|DestroyActor))

(event EventBeginPlay)

(event EventDamage
  (params (DamageAmount :type Integer))
  ;[0.1 0.1 0.1] Damage
  (bind _output_get (Variables|Default|SetLife (- (Variables|Default|GetLife) DamageAmount)))
  (if (<= _output_get 0)
    (CallFunction|DropResources)))

(fn ConstructionScript)