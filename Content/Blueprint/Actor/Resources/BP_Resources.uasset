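; BP_Resources is a resource pickup actor holding a Type and an Amount, shown through a WBP_Resource widget configured on BeginPlay.
; Pickup adds the resource to the main character's inventory widget through its HUD, then destroys the actor.
; ActivateHud shows the widget and hides it after a short retriggerable delay, so it stays visible only while the event keeps being called.
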(event EventBeginPlay
  (|CallParentFunction)
  (bind _aswbp_resource (Utilities|Casting|CastToWBP_Resource (UserInterface|GetWidget (Variables|Default|GetWidget))))
  (Default|Setup _aswbp_resource (Variables|Default|GetType) (Variables|Default|GetAmount)))

(event Collision|EventActorBeginOverlap
  (params (OtherActor :type Actor%20Object%20Reference))
  (|CallParentFunction OtherActor) ; This node is disabled and will not be called.\nDrag off pins to build functionality.
)

(event EventTick
  (params (DeltaSeconds :type Float%20%28single-precision%29))
  (|CallParentFunction DeltaSeconds))

(event EventPickup
  (params (Actor :type Actor%20Object%20Reference))
  (bind _asbp_main_character (Utilities|Casting|CastToBP_MainCharacter Actor))
  (Default|AddResources (Variables|/Game/Blueprint/Widget/Game/WBP_Hud.WBP_Hud_C|GetWBP_Inventory (Variables|/Game/Blueprint/Character/BP_MainCharacter.BP_MainCharacter_C|GetHud _asbp_main_character)) (Variables|Default|GetType) (Variables|Default|GetAmount))
  (Actor|DestroyActor))

(event EventActivateHud
  (Rendering|SetVisibility (Variables|Default|GetWidget) true false)
  (Utilities|FlowControl|RetriggerableDelay 0.2)
  (Rendering|SetVisibility (Variables|Default|GetWidget) false false))

(fn ConstructionScript
  (|CallParentFunction))