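; BP_Droppable is an actor that falls toward the first BP_Planet2 in the level and rests on surfaces facing away from it.
; Tick applies mass-independent gravity to its Sphere unless resting.
; Over 100 consecutive gravity-aligned hits trigger Rest, a DoOnce-guarded loop that periodically traces toward the planet.
; Resting holds while trace distance and normal match the contact; otherwise gravity resumes.
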(event OnComponentHit(Sphere)
  (params (HitComponent :type Primitive%20Component%20Object%20Reference) (OtherActor :type Actor%20Object%20Reference) (OtherComp :type Primitive%20Component%20Object%20Reference) (NormalImpulse :type Vector :default "0, 0, 0") (Hit :type Hit%20Result%20Structure%20%28by%20ref%29))
  (bind (_bblockinghit _binitialoverlap _time _distance _location _impactpoint _normal) (Collision|BreakHitResult Hit))
  (if (< (Math|Vector|Distance(Vector) (* _normal -1.0) (Variables|Default|GetGravityDirection)) 0.1)
    (Variables|Default|SetDistance _distance)
    (bind _result (Math|Integer|IncrementInt (Variables|Default|GetHitCount))
      (:%20%20
        (if (> _result 100)
          (CallFunction|Rest))))
    (else
      (Variables|Default|SetHitCount 0))))

(event Custom|Rest
  (Utilities|FlowControl|DoOnce false :!label _label
    (:Completed
      (Utilities|FlowControl|Delay 0.4 :!label _label_2)
      (bind (_outhit _returnvalue) (Collision|LineTraceByChannel (Transformation|GetActorLocation) (Transformation|GetActorLocation (Variables|Default|GetPlanet)) "TraceTypeQuery1" false 0 "None"))
      (if _returnvalue
        (if (and (Math|Float|NearlyEqual(Float) (.Distance (Collision|BreakHitResult _outhit)) (Variables|Default|GetDistance) 1e+01) (< (Math|Vector|Distance(Vector) (* (.Normal (Collision|BreakHitResult _outhit)) -1.0) (Variables|Default|GetGravityDirection)) 0.1))
          (Variables|Default|SetResting true)
          (goto _label_2)
          (else
            _)))
      (Variables|Default|SetResting false)
      (goto _label Reset))))

(event EventBeginPlay
  (bind _outactors (Actor|GetAllActorsOfClass "/Game/Blueprint/BP_Planet2.BP_Planet2_C"))
  (if (> (Utilities|Array|Length _outactors) 0)
    (Variables|Default|SetPlanet (Utilities|Array|Get(acopy) _outactors))))

(event EventTick
  (params (DeltaSeconds :type Float%20%28single-precision%29))
  (if (not (Variables|Default|GetResting))
    (bind _planet (Variables|Default|GetPlanet)
      (:then
        (Variables|Default|SetGravityDirection (Math|Vector|GetUnitDirection(Vector) (Transformation|GetActorLocation) (Transformation|GetActorLocation _planet)))
        (Physics|AddForce (Variables|Default|GetSphere) (* (Variables|Default|GetGravityDirection) (Variables|Default|GetGravityForce)) "None" true))
      (:else))))

(fn ConstructionScript)